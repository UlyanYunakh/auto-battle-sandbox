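; Visual actor for a game unit, showing its art and playing attack, death and selection feedback.
; Construction creates a dynamic material on the unit mesh, which receives the unit's art texture on initialization.
; An attack timeline lerps the actor toward its target with a Z lift and triggers the attack effect.
; A death timeline hides the base widget and animates the material tint, while selection toggles a border mesh.
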(event Custom|OnUnitInitialized
  (CallFunction|UpdateUnitArt))

(event EventBeginPlay
  (|CallParentFunction)
  (EventDispatchers|AssignOnInitialized (EventDispatchers|CreateEvent :!event Custom|OnUnitInitialized)))

(event EventDestroyed
  (EventDispatchers|UnbindEventfromOnInitialized (EventDispatchers|CreateEvent :!event Custom|OnUnitInitialized))
  (|CallParentFunction))

(event EventPlayDeathAnimation
  (Rendering|SetVisibility (Variables|Default|GetBaseWidget) false true)
  (bind _meshtint (Timeline|DeathTimeline PlayFromStart)
    (:Update
      (Rendering|Material|SetVectorParameterValue (Variables|Default|GetArtMaterialInst) "TintColor" (Math|Color|MakeColor _meshtint _meshtint _meshtint) :!class /Script/Engine.MaterialInstanceDynamic))
    (:Finished
      (Class|UnitActor|FinishDeathAnimation))))

(event EventPlayAttackAnimation
  (params (TargetPosition :type Vector :default "0, 0, 0"))
  (Variables|Default|SetCachedTargetPosition TargetPosition)
  (Variables|Default|SetCachedPosition (Transformation|GetActorLocation))
  (bind (_direction _positionlerpalpha _zoffsetlerp) (Timeline|AttackTimeline PlayFromStart)
    (:Update
      (Transformation|SetActorLocation (Math|Vector|Lerp(Vector) (Variables|Default|GetCachedPosition) (Variables|Default|GetCachedTargetPosition) _positionlerpalpha) false false)
      (Transformation|SetActorLocation (Math|Vector|Lerp(Vector) (Transformation|GetActorLocation) (+ (Transformation|GetActorLocation) (Math|Vector|MakeVector 0.0 0.0 5.0)) _zoffsetlerp) false false))
    (:Finished
      (Class|UnitActor|FinishAttackAnimation))
    (:ApplyDamage
      (Class|UnitActor|ApplyAttackEffect))))

(event EventUpdateSelectionHighlight
  (params (bHighlighted :type Boolean))
  (Rendering|SetVisibility (Variables|Default|GetBorderMesh) bHighlighted bHighlighted))

(fn ConstructionScript
  (CallFunction|CreateArtMaterial))

(fn CreateArtMaterial
  (bind _artmaterial (Variables|Default|GetArtMaterial))
  (Utilities|IsValid _artmaterial
    (:Is%20Valid
      (bind _returnvalue (Rendering|Material|CreateDynamicMaterialInstance (Variables|Default|GetUnitMesh) 0 _artmaterial "None" :!class /Script/Engine.PrimitiveComponent))
      (Variables|Default|SetArtMaterialInst _returnvalue))))

(fn UpdateUnitArt
  (if (and (Utilities|IsValidSoftObjectReference (Class|UnitActor|GetUnitArt)) (Utilities|IsValid (Variables|Default|GetArtMaterialInst)))
    (Rendering|Material|SetTextureParameterValue (Variables|Default|GetArtMaterialInst) "Texture" (Utilities|ResolveSoftReference (Class|UnitActor|GetUnitArt)))))